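; Arena game state that tracks remaining enemies and ends the match when all are gone.
; On BeginPlay it sets EnemyCount from the turret and walker enemies found in the level.
; UpdateEnemyCount decrements that count and opens the End_Game level once it reaches zero or below.
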(event `self.ReceiveBeginPlay`
  (bind _outactors (`GameplayStatics.GetAllActorsOfClass` "/Game/Blueprints/Enemies/Turret/BP_Enemy_Turret.BP_Enemy_Turret_C"))
  (bind _outactors_2 (`GameplayStatics.GetAllActorsOfClass` "/Game/Blueprints/Enemies/Walker/BP_Enemy_Walker.BP_Enemy_Walker_C"))
  (set `self.Enemy Count` (+ (`KismetArrayLibrary.Array_Length` _outactors_2) (`KismetArrayLibrary.Array_Length` _outactors))))

(event `Update Enemy Count`
  (bind _output_get (set `self.Enemy Count` (- (`self.Enemy Count`) 1)))
  (if (<= _output_get 0)
    (`GameplayStatics.OpenLevel` "End_Game")))

(fn `UserConstructionScript`)