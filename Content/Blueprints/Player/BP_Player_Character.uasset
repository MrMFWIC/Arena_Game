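; Player character with camera-relative movement and look, a double jump, a dash, a grappling hook and a timed melee box.
; Jumps are upward launches counted by a DoN that resets on landing; the dash hops, launches forward, then restores prior speed before a cooldown.
; Holding right mouse traces from the camera; a hit enables flying, cable display and a per-tick pull toward the impact point.
; Left click briefly activates the box component, with a cooldown.
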(event `InputAxis|Movement Forward/Reverse`
  (params (AxisValue :type "Float (single-precision)"))
  ;[1 1 1] Player Movement
  (`self.AddMovementInput` (`SceneComponent.GetForwardVector` (`self.Camera`)) AxisValue))

(event `InputAxis|Movement Strafing`
  (params (AxisValue :type "Float (single-precision)"))
  ;[1 1 1] Player Movement
  (`self.AddMovementInput` (`SceneComponent.GetRightVector` (`self.Camera`)) AxisValue))

(event `InputAxis|Horizontal Look`
  (params (AxisValue :type "Float (single-precision)"))
  ;[1 1 1] Player Look
  (`self.AddControllerYawInput` AxisValue))

(event `InputAction|Jump`
  (params (Key :type "Key Structure"))
  ;[1 1 1] Player Movement
  (:`Pressed`
    (`/Engine/EditorBlueprintResources/StandardMacros.Do N` 2 :!label _label
      (:`Exit`
        (`self.LaunchCharacter` (0.0 0.0 900.0) false true)))))

(event `InputAxis|Vertical Look`
  (params (AxisValue :type "Float (single-precision)"))
  ;[1 1 1] Player Look
  (`self.AddControllerPitchInput` AxisValue))

(event `self.OnLanded`
  (params (Hit :type "HitResult Structure (by ref)"))
  ;[1 1 1] Player Movement
  (goto _label :!via `Reset`))

(event `InputAction|Dash`
  (params (Key :type "Key Structure"))
  ;[1 1 1] Dash
  (:`Pressed`
    (`/Engine/EditorBlueprintResources/StandardMacros.DoOnce` false :!label _label_2
      (:`Completed`
        (set `self.preDashSpeed` (`KismetMathLibrary.VSize` (`MovementComponent.Velocity` (`self.CharacterMovement`))))
        (`self.LaunchCharacter` (0.0 0.0 200.0))
        (`KismetSystemLibrary.Delay` 0.1)
        (`self.LaunchCharacter` (* (`SceneComponent.GetForwardVector` (`self.CapsuleComponent`)) 12000.0))
        (bind _output_get (set `self.postDashDirection` (`KismetMathLibrary.Conv_RotatorToVector` (`CharacterMovementComponent.GetLastUpdateRotation` (`self.CharacterMovement`)))))
        (`KismetSystemLibrary.Delay` 0.2)
        (set `MovementComponent.Velocity` (* _output_get (`self.preDashSpeed`)) (`self.CharacterMovement`))
        (`KismetSystemLibrary.Delay` 1.0)
        (goto _label_2 :!via `Reset`)))))

(event `Key|RightMouseButton`
  (params (Key :type "Key Structure"))
  (bind _camera (`self.Camera`))
  (bind _returnvalue (`SceneComponent.K2_GetComponentLocation` _camera))
  ;[1 1 1] Grappling Mechanic
  (:`Pressed`
    (bind (_outhit _returnvalue_2) (`KismetSystemLibrary.LineTraceSingle` _returnvalue (+ _returnvalue (* (`KismetMathLibrary.GetForwardVector` (`SceneComponent.K2_GetComponentRotation` _camera)) (`self.GrappleHookDistance`))) "TraceTypeQuery1"))
    (if _returnvalue_2
      (set `self.hookImpactPoint` (`.ImpactPoint` (`GameplayStatics.BreakHitResult` _outhit)))
      (set `self.isGrappling` true)
      (`CharacterMovementComponent.SetMovementMode` (`self.CharacterMovement`) "MOVE_Flying" 0)
      (`SceneComponent.SetVisibility` (`self.Cable`) true false)))
  (:`Released`
    (set `self.isGrappling` false)
    (`CharacterMovementComponent.SetMovementMode` (`self.CharacterMovement`) "MOVE_Falling" 0)
    (`SceneComponent.SetVisibility` (`self.Cable`) false false)))

(event `self.ReceiveTick`
  (params (DeltaSeconds :type "Float (single-precision)"))
  ;[1 1 1] Grappling Mechanic
  (if (`self.isGrappling`)
    (set `CableComponent.EndLocation` (`KismetMathLibrary.InverseTransformLocation` (`self.GetTransform`) (`self.hookImpactPoint`)) (`self.Cable`))
    (`CharacterMovementComponent.AddForce` (`self.CharacterMovement`) (* (`KismetMathLibrary.Normal` (`KismetMathLibrary.GetDirectionUnitVector` (`self.K2_GetActorLocation`) (`self.hookImpactPoint`))) (`self.GrapplePullForce`)))))

(event `self.ReceiveBeginPlay`
  ;[1 1 1] Melee System
  (`ActorComponent.SetActive` (`self.Box`) false false))

(event `Key|LeftMouseButton`
  (params (Key :type "Key Structure"))
  ;[1 1 1] Melee System
  (:`Pressed`
    (`/Engine/EditorBlueprintResources/StandardMacros.DoOnce` false :!label _label_3
      (:`Completed`
        (`ActorComponent.SetActive` (`self.Box`) true false)
        (`KismetSystemLibrary.Delay` 0.3)
        (`ActorComponent.SetActive` (`self.Box`) false false)
        (`KismetSystemLibrary.Delay` 0.7)
        (goto _label_3 :!via `Reset`)))))

(fn `UserConstructionScript`)