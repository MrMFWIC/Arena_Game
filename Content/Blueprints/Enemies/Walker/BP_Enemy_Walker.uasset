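; BP_Enemy_Walker is an early-stage walker enemy Blueprint that detects the player through PawnSensing.
; When the sensed pawn casts to BP_Player_Character, it stores the player reference and sets a SensedPawn flag.
; Tick checks that flag but takes no action, and an unconnected look-at rotation interpolation toward the player remains unused.
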(event `self.PawnSensing.OnSeePawn`
  (params (Pawn :type "Pawn Object Reference"))
  (bind _asbp_player_character (cast `/Game/Blueprints/Player/BP_Player_Character` Pawn))
  (set `self.PlayerReference` _asbp_player_character)
  (set `self.SensedPawn` true))

(event `self.ReceiveTick`
  (params (DeltaSeconds :type "Float (single-precision)"))
  (if (`self.SensedPawn`)
    _))

(fn `UserConstructionScript`)